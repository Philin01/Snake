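; BP_Snake is the player snake Blueprint that adds end-of-game screens and sounds on top of its parent class.
; It overrides the restart-level and win-game widget events, calling the parent version first.
; Losing clears all widgets, shows the lost widget and plays a 2D lose sound.
; Winning does the same with the win widget and sound, but only when IsWin is set.
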(event `self.ReceiveTick`
  (params (DeltaSeconds :type "Float (single-precision)")))

(event `self.AddWidgetRestartLevel`
  (`parent.AddWidgetRestartLevel`)
  (`WidgetLayoutLibrary.RemoveAllWidgets`)
  (bind _returnvalue (`|CreateWidget` "/Game/Blueprints/UI/WBP_LostWidget.WBP_LostWidget_C"))
  (`UserWidget.AddToViewport` _returnvalue 0)
  (`GameplayStatics.PlaySound2D` "/Game/Assets/Sounds/S_LostSound.S_LostSound" 1.0 1.0 0.0 null null))

(event `self.AddWidgetWinGame`
  (`parent.AddWidgetWinGame`)
  (if (`self.bIsWin`)
    (`WidgetLayoutLibrary.RemoveAllWidgets`)
    (bind _returnvalue (`|CreateWidget` "/Game/Blueprints/UI/WBP_WinWidget.WBP_WinWidget_C"))
    (`UserWidget.AddToViewport` _returnvalue 0)
    (`GameplayStatics.PlaySound2D` "/Game/Assets/Sounds/S_WinSoundCue.S_WinSoundCue" 1.0 1.0 0.0 null null)))

(fn `UserConstructionScript`)